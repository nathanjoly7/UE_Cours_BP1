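; A lamp Blueprint whose SpotLight is toggled by an event from a PlaqueSendEvent reference, by its name likely a pressure plate.
; On BeginPlay it binds ToggleLight to that object's ActivateStuff dispatcher.
; ToggleLight uses a FlipFlop to alternate the light's visibility, starting with on, prints the flip state and applies the Lightcolor variable to the light.
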(event Custom|ToggleLight
  (bind _isa (Utilities|FlowControl|FlipFlop)
    (:A
      (Rendering|SetVisibility (Variables|Default|GetSpotLight) true false))
    (:B
      (Rendering|SetVisibility (Variables|Default|GetSpotLight) false false)))
  (Development|PrintString (Utilities|String|ToString(Boolean) _isa))
  (Rendering|Components|Light|SetLightColor (Variables|Default|GetSpotLight) (Math|Conversions|ToLinearColor(Color) (Variables|Default|Getlightcolor)) true))

(event EventBeginPlay
  (EventDispatchers|BindEventtoActivateStuff (Variables|Default|GetPlaqueSendEvent) (delegate Custom|ToggleLight)))

(fn ConstructionScript)