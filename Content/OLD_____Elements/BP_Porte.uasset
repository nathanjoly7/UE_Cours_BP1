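; Door Blueprint that toggles open and closed by swinging its mesh on yaw each time it is activated.
; Activate calls OpenDoor, where a FlipFlop alternates between playing one timeline forward and a second timeline in reverse from its end.
; Each timeline lerps the mesh's relative yaw between two angle variables and sets collision to query and physics on every update.
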(event Custom|OpenDoor
  (Utilities|FlowControl|FlipFlop
    (:A
      (bind _newtrack_0 (Timeline|Timeline PlayFromStart)
        (:Update
          (Transformation|SetRelativeRotation (Variables|Default|GetDoorMesh) (Math|Rotator|MakeRotator 0.0 0.0 (Math|Float|Lerp (Variables|Default|Getdooropenfloat) (Variables|Default|Getdoorclosefloat_0) _newtrack_0)) false false)
          (Collision|SetCollisionEnabled (Variables|Default|GetDoorMesh) "QueryAndPhysics"))))
    (:B
      (bind _newtrack_0_2 (Timeline|Timeline_0 ReverseFromEnd)
        (:Update
          (Transformation|SetRelativeRotation (Variables|Default|GetDoorMesh) (Math|Rotator|MakeRotator 0.0 0.0 (Math|Float|Lerp (Variables|Default|Getdooropenfloat) (Variables|Default|Getdoorclosefloat_0) _newtrack_0_2)) false false)
          (Collision|SetCollisionEnabled (Variables|Default|GetDoorMesh) "QueryAndPhysics"))))))

(event EventActivate
  (CallFunction|OpenDoor))

(fn ConstructionScript)