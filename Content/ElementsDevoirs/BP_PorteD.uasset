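; BP_PorteD is a door Blueprint that swings open or closed when it receives the Activate interface event.
; OpenDoor toggles on IsOpened, driving timelines that lerp the mesh yaw and update that flag, and BeginPlay plays the opening if the flag starts true.
; Add1 and Substract1 still update an open-door count, noted as an obsolete system broken by per-instance values.
; Bindings to three switches are left unconnected.
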(event Custom|OpenDoor
  (if (Variables|Default|GetIs%20Opened%20?)
    (Utilities|FlowControl|Sequence
      (:then_0
        ;[1 1 1] animation fermeture
        (bind _newtrack_0 (Timeline|Timeline_0 ReverseFromEnd)
          (:Update
            (Transformation|SetRelativeRotation (Variables|Default|GetDoorMesh) (Math|Rotator|MakeRotator 0.0 0.0 (Math|Float|Lerp (Variables|Default|Getdooropenfloat) (Variables|Default|Getdoorclosefloat_0) _newtrack_0)) false false)
            (Collision|SetCollisionEnabled (Variables|Default|GetDoorMesh) "QueryAndPhysics")
            (Variables|Default|SetIs%20Opened%20? false))))
      (:then_1
        ;[1 1 1] ancien systeme comptage portes ouvertes. Ne marche pas car le blueprint est unique mais il y a trois portes, donc la variable a trois valeurs différente en même temps
        (Utilities|Substract1)))
    (else
      (Utilities|FlowControl|Sequence
        (:then_0
          ;[1 1 1] Animation ouverture porte
          (bind _newtrack_0_2 (Timeline|Timeline PlayFromStart)
            (:Update
              (Transformation|SetRelativeRotation (Variables|Default|GetDoorMesh) (Math|Rotator|MakeRotator 0.0 0.0 (Math|Float|Lerp (Variables|Default|Getdooropenfloat) (Variables|Default|Getdoorclosefloat_0) _newtrack_0_2)) false false)
              (Collision|SetCollisionEnabled (Variables|Default|GetDoorMesh) "QueryAndPhysics")
              (Variables|Default|SetIs%20Opened%20? true))))
        (:then_1
          (Utilities|Add1))))))

(event EventActivate
  ;[1 1 1] quand je reçois l'event de l'interface, j'appelle  mon event qui ouvre / ferme
  (CallFunction|OpenDoor))

(event EventBeginPlay
  (if (Variables|Default|GetIs%20Opened%20?)
    ;[1 1 1] Animation ouverture porte
    (bind _newtrack_0 (Timeline|Timeline PlayFromStart)
      (:Update
        (Transformation|SetRelativeRotation (Variables|Default|GetDoorMesh) (Math|Rotator|MakeRotator 0.0 0.0 (Math|Float|Lerp (Variables|Default|Getdooropenfloat) (Variables|Default|Getdoorclosefloat_0) _newtrack_0)) false false)
        (Collision|SetCollisionEnabled (Variables|Default|GetDoorMesh) "QueryAndPhysics")
        (Variables|Default|SetIs%20Opened%20? true)))))

(fn ConstructionScript)