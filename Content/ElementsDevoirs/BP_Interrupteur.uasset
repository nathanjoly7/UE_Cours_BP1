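; BP_Interrupteur is a secondary switch that activates connected actors, such as doors, once the main switch has enabled it.
; On BeginPlay it binds to InterrPrincipal, whose event sets the PrincipalIsEnabled flag that gates both prompt and interaction.
; Collision overlaps by the third-person character show or hide the widget.
; Interact sends ActivateMessage to every ActorsReceivers entry implementing BPI_Interrupteurs.
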(event OnComponentBeginOverlap(collision)
  (params (OverlappedComponent :type Primitive%20Component%20Object%20Reference) (OtherActor :type Actor%20Object%20Reference) (OtherComp :type Primitive%20Component%20Object%20Reference) (OtherBodyIndex :type Integer) (bFromSweep :type Boolean) (SweepResult :type Hit%20Result%20Structure%20%28by%20ref%29))
  ;[1 1 1] afficher / masquer widget
  (Utilities|Casting|CastToBP_ThirdPersonCharacter OtherActor)
  (if (Variables|Default|GetPrincipalIsEnabled?)
    (Rendering|SetVisibility (Variables|Default|GetWidget) true false)))

(event OnComponentEndOverlap(collision)
  (params (OverlappedComponent :type Primitive%20Component%20Object%20Reference) (OtherActor :type Actor%20Object%20Reference) (OtherComp :type Primitive%20Component%20Object%20Reference) (OtherBodyIndex :type Integer))
  ;[1 1 1] afficher / masquer widget
  (Utilities|Casting|CastToBP_ThirdPersonCharacter OtherActor)
  (if (Variables|Default|GetPrincipalIsEnabled?)
    (Rendering|SetVisibility (Variables|Default|GetWidget) false false)))

(event Custom|ActiverUtilisation
  (params (Active :type Boolean))
  ;[1 1 1] si on reçoit l'event de l'interrupteur principal, on active la possiblité d'activer les interr. secondaires
  (Variables|Default|SetPrincipalIsEnabled? Active))

(event EventBeginPlay
  ;[1 1 1] si on reçoit l'event de l'interrupteur principal, on active la possiblité d'activer les interr. secondaires
  (EventDispatchers|BindEventtoActivateOtherInterruptors (Variables|Default|GetInterrPrincipal) (delegate Custom|ActiverUtilisation)))

(event EventInteract
  ;[1 1 1] quand je recois l'event interact j'envoie l'event "activate" au portes connectées
  (if (Variables|Default|GetPrincipalIsEnabled?)
    (for _array_element (Variables|Default|GetActorsReceivers)
      (if (Utilities|DoesObjectImplementInterface _array_element "/Game/BPI_Interrupteurs.BPI_Interrupteurs_C")
        (Class|BPIInterrupteurs|Activate(Message) _array_element)))))

(fn ConstructionScript)