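; BP_Lampe is a lamp that lights its SpotLight once three doors are all reported closed.
; On BeginPlay it binds to door-closed dispatchers on three Detection references, each storing its state in a Test boolean.
; Every update runs TestDoors, which waits briefly, then turns the light on if all three booleans are true.
; Nothing turns the light off again, and a debug print of the states is left unconnected.
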(event Custom|TurnOn
  (Rendering|SetVisibility (Variables|Default|GetSpotLight) true false))

(event Custom|Door3closed
  (params (Closed3 :type Boolean))
  (Variables|Default|Settest3 Closed3)
  (CallFunction|TestDoors))

(event Custom|Door1closed
  (params (Closed1 :type Boolean))
  (Variables|Default|Settest1 Closed1)
  (CallFunction|TestDoors))

(event Custom|Door2closed
  (params (Closed2 :type Boolean))
  (Variables|Default|Settest2 Closed2)
  (CallFunction|TestDoors))

(event Custom|TestDoors
  (Utilities|FlowControl|Delay 0.2)
  (if (Variables|Default|Gettest1)
    (if (Variables|Default|Gettest2)
      (if (Variables|Default|Gettest3)
        (CallFunction|Turnon)))))

(event EventBeginPlay
  (EventDispatchers|BindEventtoDoorClosed1 (Variables|Default|GetDetection1) (delegate Custom|Door1closed))
  (EventDispatchers|BindEventtoDoorClosed2 (Variables|Default|GetDetection2) (delegate Custom|Door2closed))
  (EventDispatchers|BindEventtoDoorClosed3 (Variables|Default|GetDetection3) (delegate Custom|Door3closed)))

(event EventTick
  (params (DeltaSeconds :type Float%20%28single-precision%29))
  ;[1 1 1] Tests Debugging
)

(fn ConstructionScript)